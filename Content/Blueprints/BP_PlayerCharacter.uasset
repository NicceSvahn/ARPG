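; Player character Blueprint that delegates health to a HealthComponent and handles the character's death.
; On death it stops movement immediately, plays a non-looping death animation on the mesh, then destroys the actor after a short delay.
; Hardcoded T and R keys directly apply damage and healing through the component.
; The health-changed event is bound but empty.
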(event `self.HealthComponent.OnHealthChanged`
  (params (NewHealth :type "Float (single-precision)")))

(event `self.HealthComponent.OnDeath`
  (`MovementComponent.StopMovementImmediately` (`self.CharacterMovement`))
  (`SkeletalMeshComponent.PlayAnimation` (`self.Mesh`) "/Game/Characters/Mannequins/Anims/Death/MM_Death_Back_01.MM_Death_Back_01" false)
  (`KismetSystemLibrary.Delay` 3.0)
  (`self.K2_DestroyActor`))

(event `Key|T`
  (params (Key :type "Key Structure"))
  (:`Pressed`
    (`HealthComponent.TakeDamage` (`self.HealthComponent`) 25.0)))

(event `Key|R`
  (params (Key :type "Key Structure"))
  (:`Pressed`
    (`HealthComponent.Heal` (`self.HealthComponent`) 10.0)))

(fn `UserConstructionScript`)